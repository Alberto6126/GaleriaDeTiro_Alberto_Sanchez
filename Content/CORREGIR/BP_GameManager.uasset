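; BP_GameManager tracks the player's score and runs a countdown that starts when a rifle pickup is collected.
; On BeginPlay it binds WeaponPicked to OnCollectedWeapon on the first BP_Pickup_Rifle found in the level.
; WeaponPicked loops through a one-second Delay, printing and decrementing CountdownTimer until it prints "END" at zero.
; AddScore updates Score and calls PrintScore, which prints the gained and total points in green Spanish text.
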(event `self.ReceiveBeginPlay`
  ;[1 1 1] Comunicar arma con game manager y escuchar el evento OnCollectedWeapon
  (bind _outactors (`GameplayStatics.GetAllActorsOfClass` "/Game/FirstPerson/Blueprints/BP_Pickup_Rifle.BP_Pickup_Rifle_C"))
  (add `/Game/FirstPerson/Blueprints/BP_Pickup_Rifle.onCollectedWeapon` (`|GetArrayItem` _outactors) (delegate `WeaponPicked`)))

(event `WeaponPicked`
  ;[1 1 1] Comunicar arma con game manager y escuchar el evento OnCollectedWeapon
  ;[1 1 1] Gestión del timer
  (`KismetSystemLibrary.Delay` 1.0 :!label _label)
  (`KismetSystemLibrary.PrintString` (`KismetStringLibrary.Conv_IntToString` (`self.CountdownTimer`)))
  (if (== (`self.CountdownTimer`) 0)
    (`KismetSystemLibrary.PrintString` "END")
    (else
      (`/Engine/EditorBlueprintResources/StandardMacros.DecrementInt` (`self.CountdownTimer`)
        (:`  `
          (goto _label))))))

(fn `AddScore`
  (params (ScoreToAdd :type Integer))
  (bind _score (`self.Score`))
  (set `self.Score` (+ ScoreToAdd _score))
  (`self.PrintScore` ScoreToAdd _score))

(fn `UserConstructionScript`)