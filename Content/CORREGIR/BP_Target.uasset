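; BP_Target is a moving shooting-gallery target that awards score when shot.
; Tick slides DianaMesh along Direction at RowSpeed, with SetInversion choosing the sign (false negates Direction).
; A hit from BP_FirstPersonProjectile destroys the projectile, spawns an explosion, adds Score to the BP_GameManager found at BeginPlay, then destroys the target.
; Actor overlap only prints a debug message.
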(event `self.ReceiveHit`
  (params (MyComp :type "PrimitiveComponent Object Reference") (Other :type "Actor Object Reference") (OtherComp :type "PrimitiveComponent Object Reference") (bSelfMoved :type Boolean) (HitLocation :type "Vector Structure") (HitNormal :type "Vector Structure") (NormalImpulse :type "Vector Structure") (Hit :type "HitResult Structure (by ref)"))
  (bind _asbp_first_person_projectile (cast `/Game/FirstPerson/Blueprints/BP_FirstPersonProjectile` Other))
  (`self.K2_DestroyActor` _asbp_first_person_projectile)
  (`GameplayStatics.SpawnEmitterAtLocation` "/Game/StarterContent/Particles/P_Explosion.P_Explosion" HitLocation)
  (`/Game/CORREGIR/BP_GameManager.AddScore` (`self.GameManagerRef`) (`self.Score`))
  (`self.K2_DestroyActor`))

(event `self.ReceiveBeginPlay`
  (bind _outactors (`GameplayStatics.GetAllActorsOfClass` "/Game/CORREGIR/BP_GameManager.BP_GameManager_C"))
  (set `self.GameManagerRef` (`|GetArrayItem` _outactors)))

(event `self.ReceiveActorBeginOverlap`
  (params (OtherActor :type "Actor Object Reference"))
  (`KismetSystemLibrary.PrintText` "Colision"))

(event `self.ReceiveTick`
  (params (DeltaSeconds :type "Float (single-precision)"))
  (bind _dianamesh (`self.DianaMesh`))
  (bind _returnvalue (* (* DeltaSeconds (`self.RowSpeed`)) (`self.Direction`)))
  (if (`self.isInverted`)
    (`SceneComponent.K2_AddWorldOffset` _dianamesh _returnvalue false true)
    (else
      (`SceneComponent.K2_AddWorldOffset` _dianamesh (* _returnvalue (-1.0 -1.0 -1.0)) false false))))

(fn `setInversion`
  (params (inversion :type Boolean))
  (set `self.isInverted` inversion))

(fn `UserConstructionScript`)