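; BP_Zone is a trigger actor that reports whether the player has won or lost on entering it.
; On BeginPlay it caches the first BP_GameManager found in the level.
; When BP_FirstPersonCharacter overlaps it, it fires the OnZoneEntered dispatcher, then compares the manager's Score to WinScore.
; It prints a Spanish result with score and margin, green for a win or red for a loss, with ties counting as losses.
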(event `self.ReceiveBeginPlay`
  (bind _outactors (`GameplayStatics.GetAllActorsOfClass` "/Game/CORREGIR/Blueprints/BP_GameManager.BP_GameManager_C"))
  (set `self.GameManagerRef` (`|GetArrayItem` _outactors)))

(event `self.ReceiveActorBeginOverlap`
  (params (OtherActor :type "Actor Object Reference"))
  ;[1 0.9256 0.6461] Al haber un overlap se revisa si el actor es el personaje
  (cast `/Game/FirstPerson/Blueprints/BP_FirstPersonCharacter` OtherActor)
  ;[0.4696 0.8276 1] En el caso de que lo sea, se llama al evento Zone Entered y se imprimen los scores
  (`self.onZoneEntered`)
  (`self.ScoreStatePrint`))

(fn `UserConstructionScript`)